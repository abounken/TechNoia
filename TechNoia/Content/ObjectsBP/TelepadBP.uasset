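; TelepadBP is a telepad actor meant to send the player character to another pad, paired by Destination and PortalID.
; Any overlap on its Sphere searches all TelepadBP actors for a PortalID matching its Destination, without checking which actor overlapped.
; On each match it teleports player 0's TopDownCharacter to a zero location and rotation; the matched pad's transform is not used.
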(event `self.ReceiveTick`
  (params (DeltaSeconds :type "Float (single-precision)")))

(event `self.Sphere.OnComponentBeginOverlap`
  (params (OverlappedComponent :type "PrimitiveComponent Object Reference") (OtherActor :type "Actor Object Reference") (OtherComp :type "PrimitiveComponent Object Reference") (OtherBodyIndex :type Integer) (bFromSweep :type Boolean) (SweepResult :type "HitResult Structure (by ref)"))
  (bind _outactors (`GameplayStatics.GetAllActorsOfClass` "TelepadBP_C"))
  (for (_array_element _array_index) _outactors
    (bind _astelepad_bp (cast `/Game/ObjectsBP/TelepadBP` _array_element))
    (if (`KismetStringLibrary.EqualEqual_StrStr` (`self.Destination`) (`/Game/ObjectsBP/TelepadBP.PortalID` _astelepad_bp))
      (bind _astop_down_character (cast `/Game/TopDownBP/Blueprints/TopDownCharacter` (`GameplayStatics.GetPlayerCharacter` 0)))
      (`self.K2_TeleportTo` :`self` _astop_down_character))))

(fn `UserConstructionScript`)