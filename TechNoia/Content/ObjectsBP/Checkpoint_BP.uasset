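; Checkpoint actor that saves the player's progress the first time the player reaches it.
; An overlap on its Sphere fires only for the FirstPersonCharacter's capsule component, and a CheckpointActivated flag makes it one-shot.
; On activation it calls StoreCheckpointLocation on the TechNoia_GI game instance, then swaps the Cube's material to a glow outline as visual feedback.
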(event `self.Sphere.OnComponentBeginOverlap`
  (params (OverlappedComponent :type "PrimitiveComponent Object Reference") (OtherActor :type "Actor Object Reference") (OtherComp :type "PrimitiveComponent Object Reference") (OtherBodyIndex :type Integer) (bFromSweep :type Boolean) (SweepResult :type "HitResult Structure (by ref)"))
  (if (not (`self.CheckpointActivated`))
    (bind _asfirst_person_character (cast `/Game/FirstPersonBP/Blueprints/FirstPersonCharacter` OtherActor))
    (if (== (`Character.CapsuleComponent` _asfirst_person_character) OtherComp)
      (set `self.CheckpointActivated` true)
      (bind _astech_noia_gi (cast `/Game/TechNoia_GI` (`GameplayStatics.GetGameInstance`)))
      (`/Game/TechNoia_GI.StoreCheckpointLocation` _astech_noia_gi)
      (`PrimitiveComponent.SetMaterial` (`self.Cube`) 0 "/Game/Outline/Materials/GlowOutline_Inst.GlowOutline_Inst"))))

(fn `UserConstructionScript`)