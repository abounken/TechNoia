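; Security camera that sweeps its view cone, tracks the player and can trigger real-world game over when the cone overlaps the player's capsule.
; Tick checks line of sight and range, then optionally stops the sweeps, aims Camera03 yaw and Camera04 roll at the player and turns the cone red.
; Otherwise optional side and up-down timelines drive the sweep, with reverse options.
; Construction script sizes the cone; PawnSensing only prints debug text.
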(event `self.ReceiveBeginPlay`
  (set `self.InitialRotation` (`self.K2_GetActorRotation`)))

(event `self.PawnSensing.OnSeePawn`
  (params (Pawn :type "Pawn Object Reference"))
  (`KismetSystemLibrary.PrintString` "Sensed" :!label _label))

(event `self.PawnSensing.OnComponentActivated`
  (params (Component :type "ActorComponent Object Reference") (bReset :type Boolean))
  (goto _label))

(event `self.PawnSensing1.OnSeePawn`
  (params (Pawn :type "Pawn Object Reference"))
  (goto _label))

(event `self.CameraCone.OnComponentBeginOverlap`
  (params (OverlappedComponent :type "PrimitiveComponent Object Reference") (OtherActor :type "Actor Object Reference") (OtherComp :type "PrimitiveComponent Object Reference") (OtherBodyIndex :type Integer) (bFromSweep :type Boolean) (SweepResult :type "HitResult Structure (by ref)"))
  (if (`self.KillPlayer`)
    (bind _asfirst_person_character (cast `/Game/FirstPersonBP/Blueprints/FirstPersonCharacter` OtherActor))
    (if (== (`Character.CapsuleComponent` _asfirst_person_character) OtherComp)
      (bind _astech_noia_gi (cast `/Game/TechNoia_GI` (`GameplayStatics.GetGameInstance`)))
      (`/Game/TechNoia_GI.GameOverRealWorld` _astech_noia_gi)
      (`KismetSystemLibrary.PrintString` "GameIsOver"))))

(event `UpDownRotation`
  (bind _camera04 (`self.camera04`))
  (bind _camera04_2 (`self.camera04`))
  (bind (_relativerotation_roll _relativerotation_pitch _relativerotation_yaw) (`KismetMathLibrary.BreakRotator` (`SceneComponent.RelativeRotation` _camera04_2)))
  ;[1 1 1] UPDOWN
  (bind (_direction _rot) (`Timeline|Timeline_0` :`NewTime` 0.2 :!label _label_2)
    (:`Update`
      (if (`self.ReverseUpDown`)
        (`SceneComponent.K2_SetRelativeRotation` _camera04 (`KismetMathLibrary.MakeRotator` (* _rot -1.0) _relativerotation_pitch _relativerotation_yaw) false false)
        (else
          (`SceneComponent.K2_SetRelativeRotation` _camera04 (`KismetMathLibrary.RInterpTo` (`SceneComponent.RelativeRotation` _camera04_2) (`KismetMathLibrary.MakeRotator` _rot _relativerotation_pitch _relativerotation_yaw) (`self.DeltaSeconds`) 3.0) false false))))))

(event `self.ReceiveTick`
  (params (DeltaSeconds :type "Float (single-precision)"))
  (bind _returnvalue (`GameplayStatics.GetPlayerPawn` 0))
  (bind _returnvalue_2 (`self.K2_GetActorLocation`))
  (bind _cameracone (`self.CameraCone`))
  (bind _returnvalue_3 (`self.K2_GetActorLocation` _returnvalue))
  (bind (_relativerotation_roll _relativerotation_pitch _relativerotation_yaw) (`KismetMathLibrary.BreakRotator` (`SceneComponent.RelativeRotation` (`self.camera03`))))
  (bind (_relativerotation_roll_2 _relativerotation_pitch_2 _relativerotation_yaw_2) (`KismetMathLibrary.BreakRotator` (`SceneComponent.RelativeRotation` (`self.camera04`))))
  (bind (_returnvalue_roll _returnvalue_pitch) (`KismetMathLibrary.BreakRotator` (`KismetMathLibrary.FindLookAtRotation` (`self.K2_GetActorLocation`) (`self.K2_GetActorLocation` (`GameplayStatics.GetPlayerCharacter` 0)))))
  (bind (_returnvalue_roll_2 _returnvalue_pitch_2 _returnvalue_yaw) (`KismetMathLibrary.BreakRotator` (`KismetMathLibrary.FindLookAtRotation` (`self.K2_GetActorLocation`) (`self.K2_GetActorLocation` (`GameplayStatics.GetPlayerCharacter` 0)))))
  (bind (_returnvalue_roll_3 _returnvalue_pitch_3 _returnvalue_yaw_2) (`KismetMathLibrary.BreakRotator` (`KismetMathLibrary.RInterpTo` (`KismetMathLibrary.MakeRotator` 0.0 0.0 _relativerotation_yaw) (`KismetMathLibrary.MakeRotator` 0.0 0.0 (+ _returnvalue_yaw 90.0)) (`GameplayStatics.GetWorldDeltaSeconds`) 3.0)))
  (set `self.DeltaSeconds` DeltaSeconds)
  (`/Engine/EditorBlueprintResources/StandardMacros.IsValid` _returnvalue
    (:`Is Valid`
      ;[1 1 1] Player In Range?
      (bind _outhit (`KismetSystemLibrary.LineTraceSingle` :`Start` _returnvalue_2 :`End` _returnvalue_3 :`TraceChannel` "TraceTypeQuery1" :`DrawDebugType` "ForOneFrame"))
      (if (== (`.HitActor` (`GameplayStatics.BreakHitResult` _outhit)) (`GameplayStatics.GetPlayerCharacter` 0))
        (set `self.PlayerSeen` true)
        (else
          (set `self.PlayerSeen` false)))
      (set `self.PlayerInRange` (<= (`KismetMathLibrary.VSize` (- _returnvalue_3 _returnvalue_2)) (`self.TargetRange`)))
      (if (and (`self.PlayerSeen`) (`self.PlayerInRange`))
        (if (`self.CanTargetPlayer`)
          (`self.StopManual`)
          ;[1 1 1] YAW and CAM03
          (`SceneComponent.K2_SetRelativeRotation` (`self.camera03`) (`KismetMathLibrary.MakeRotator` _relativerotation_roll _relativerotation_pitch _returnvalue_yaw_2) false false)
          (`self.StopManualSide`)
          ;[1 1 1] ROLL and CAM04
          (`SceneComponent.K2_SetRelativeRotation` (`self.camera04`) (`KismetMathLibrary.MakeRotator` (* _returnvalue_pitch -1.0) _returnvalue_roll _relativerotation_yaw_2) false false)
          (`PrimitiveComponent.SetMaterial` (`self.CameraCone`) 0 "/Game/ObjectsBP/CameraGradient_Red.CameraGradient_Red"))
        (else
          (`|ExecutionSequence`
            (:`then_0`
              (if (`self.CanTargetPlayer`)
                (`PrimitiveComponent.SetMaterial` _cameracone 0 "/Game/ObjectsBP/CameraGradient_Blue.CameraGradient_Blue")
                (`PrimitiveComponent.SetMaterial` _cameracone 1 "/Game/ObjectsBP/CameraGradient_Blue.CameraGradient_Blue"))
              (if (`self.RotateSide`)
                (`self.SideRotation`))
              (if (`self.RotateUpDown`)
                (`self.UpDownRotation`)))))))))

(event `SideRotation`
  (bind _camera03 (`self.camera03`))
  (bind (_relativerotation_roll _relativerotation_pitch _relativerotation_yaw) (`KismetMathLibrary.BreakRotator` (`SceneComponent.RelativeRotation` (`self.camera03`))))
  ;[1 1 1] SIDE
  (bind (_direction _rot) (`Timeline|Timeline_1` :`NewTime` 0.2 :!label _label_3)
    (:`Update`
      (if (`self.ReverseSide`)
        (`SceneComponent.K2_SetRelativeRotation` _camera03 (`KismetMathLibrary.MakeRotator` _relativerotation_roll _relativerotation_pitch (+ (* _rot -1.0) 90.0)) false false)
        (else
          (bind (_returnvalue_roll _returnvalue_pitch _returnvalue_yaw) (`KismetMathLibrary.BreakRotator` (`KismetMathLibrary.RInterpTo` (`KismetMathLibrary.MakeRotator` 0.0 0.0 _relativerotation_yaw) (`KismetMathLibrary.MakeRotator` 0.0 0.0 (+ _rot 90.0)) (`GameplayStatics.GetWorldDeltaSeconds`) 3.0)))
          (`SceneComponent.K2_SetRelativeRotation` _camera03 (`KismetMathLibrary.MakeRotator` _relativerotation_roll _relativerotation_pitch _returnvalue_yaw) false false))))))

(event `StopManualSide`
  ;[1 1 1] UPDOWN
  (goto _label_2 :!via `Stop`))

(event `StopManual`
  ;[1 1 1] SIDE
  (goto _label_3 :!via `Stop`))

(fn `UserConstructionScript`
  (bind _returnvalue (`KismetMathLibrary.FClamp` (`self.ConeRadius`) 1.0 30.0))
  (`SceneComponent.SetRelativeScale3D` (`self.CameraCone`) (`KismetMathLibrary.MakeVector` _returnvalue _returnvalue (`KismetMathLibrary.FClamp` (`self.ConeLength`) 5.0 30.0))))