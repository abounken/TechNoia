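; Level terminal actor that serves as the player's gateway to a numbered TekVoid level, unlocked in sequence.
; Completed terminals, per TechNoia_GI progress, destroy their LockedArea and show a done widget on BeginPlay.
; Sphere overlap registers the terminal as the character's ClosestTerminal and prompts if next in line; both widgets yaw toward the camera each Tick.
; OpenTerminal stores level and player/checkpoint locations, then opens the next level (call marked DISABLED).
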(event `self.ReceiveBeginPlay`
  (bind _astech_noia_gi (cast `/Game/TechNoia_GI` (`GameplayStatics.GetGameInstance`)))
  (if (>= (`/Game/TechNoia_GI.LastTerminalCompleted` _astech_noia_gi) (`self.Level`))
    (`PrimitiveComponent.SetCustomDepthStencilValue` (`self.Cube`) 0)
    (`self.K2_DestroyActor` (`self.LockedArea`))
    (`SceneComponent.SetHiddenInGame` (`self.WidgetDone`) false false)
    (`SceneComponent.SetHiddenInGame` (`self.Widget`) true false)))

(event `self.ReceiveTick`
  (params (DeltaSeconds :type "Float (single-precision)"))
  (`self.WidgetTurn`))

(event `Key|F`
  (params (Key :type "Key Structure"))
  (:`Pressed`
    (`/Engine/EditorBlueprintResources/StandardMacros.Gate` true
      (:`Exit`
        (`KismetSystemLibrary.PrintString` "Hello")))))

(event `OpenTerminal`
  (bind _astech_noia_gi (cast `/Game/TechNoia_GI` (`GameplayStatics.GetGameInstance`)))
  (set `/Game/TechNoia_GI.CurrentLevel` (`self.Level`) _astech_noia_gi)
  (`/Game/TechNoia_GI.StoreLastPlayerLocation` _astech_noia_gi)
  (`/Game/TechNoia_GI.StoreCheckpointLocation` _astech_noia_gi)
  (if (== (+ (`/Game/TechNoia_GI.LastTerminalCompleted` _astech_noia_gi) 1) (`self.Level`))
    (`GameplayStatics.OpenLevel` (`KismetStringLibrary.Conv_StringToName` (`KismetStringLibrary.Concat_StrStr` "TekVoid_0" (`KismetStringLibrary.Conv_IntToString` (`self.Level`)))))))

(event `self.Sphere.OnComponentBeginOverlap`
  (params (OverlappedComponent :type "PrimitiveComponent Object Reference") (OtherActor :type "Actor Object Reference") (OtherComp :type "PrimitiveComponent Object Reference") (OtherBodyIndex :type Integer) (bFromSweep :type Boolean) (SweepResult :type "HitResult Structure (by ref)"))
  (if (`KismetMathLibrary.ClassIsChildOf` (`GameplayStatics.GetObjectClass` OtherActor) "/Game/FirstPersonBP/Blueprints/FirstPersonCharacter.FirstPersonCharacter_C")
    (bind _asfirst_person_character (cast `/Game/FirstPersonBP/Blueprints/FirstPersonCharacter` OtherActor))
    (set `/Game/FirstPersonBP/Blueprints/FirstPersonCharacter.ClosestTerminal` self _asfirst_person_character)
    (bind _astech_noia_gi (cast `/Game/TechNoia_GI` (`GameplayStatics.GetGameInstance`)))
    (bind _lastterminalcompleted (`/Game/TechNoia_GI.LastTerminalCompleted` _astech_noia_gi))
    (if (== (+ _lastterminalcompleted 1) (`self.Level`))
      (`SceneComponent.SetHiddenInGame` (`self.Widget`) false false)
      (`KismetSystemLibrary.PrintString` (`KismetStringLibrary.Conv_IntToString` _lastterminalcompleted))
      (`KismetSystemLibrary.PrintString` (`KismetStringLibrary.Conv_IntToString` (`self.Level`))))))

(event `self.Sphere.OnComponentEndOverlap`
  (params (OverlappedComponent :type "PrimitiveComponent Object Reference") (OtherActor :type "Actor Object Reference") (OtherComp :type "PrimitiveComponent Object Reference") (OtherBodyIndex :type Integer))
  (if (`KismetMathLibrary.ClassIsChildOf` (`GameplayStatics.GetObjectClass` OtherActor) "/Game/FirstPersonBP/Blueprints/FirstPersonCharacter.FirstPersonCharacter_C")
    (bind _asfirst_person_character (cast `/Game/FirstPersonBP/Blueprints/FirstPersonCharacter` OtherActor))
    (set `/Game/FirstPersonBP/Blueprints/FirstPersonCharacter.ClosestTerminal` null _asfirst_person_character)
    (`SceneComponent.SetHiddenInGame` (`self.Widget`) true false)))

(event `self.Sphere1.OnComponentBeginOverlap`
  (params (OverlappedComponent :type "PrimitiveComponent Object Reference") (OtherActor :type "Actor Object Reference") (OtherComp :type "PrimitiveComponent Object Reference") (OtherBodyIndex :type Integer) (bFromSweep :type Boolean) (SweepResult :type "HitResult Structure (by ref)"))
  (if (`KismetMathLibrary.ClassIsChildOf` (`GameplayStatics.GetObjectClass` OtherActor) "/Game/FirstPersonBP/Blueprints/FirstPersonCharacter.FirstPersonCharacter_C")
    _))

(event `self.Sphere1.OnComponentEndOverlap`
  (params (OverlappedComponent :type "PrimitiveComponent Object Reference") (OtherActor :type "Actor Object Reference") (OtherComp :type "PrimitiveComponent Object Reference") (OtherBodyIndex :type Integer))
  (if (`KismetMathLibrary.ClassIsChildOf` (`GameplayStatics.GetObjectClass` OtherActor) "/Game/FirstPersonBP/Blueprints/FirstPersonCharacter.FirstPersonCharacter_C")
    _))

(event `WidgetTurn`
  (bind _widget (`self.Widget`))
  (bind _widgetdone (`self.WidgetDone`))
  (`SceneComponent.K2_AddLocalRotation` _widget (struct :`Yaw` 0.4) false false)
  (`SceneComponent.K2_SetWorldRotation` _widget (`KismetMathLibrary.MakeRotator` 0.0 0.0 (.yaw (`KismetMathLibrary.FindLookAtRotation` (`SceneComponent.K2_GetComponentLocation` _widget) (`self.K2_GetActorLocation` (`GameplayStatics.GetPlayerCameraManager` 0))))) false false)
  (`SceneComponent.K2_AddLocalRotation` _widgetdone (struct :`Yaw` 0.4) false false)
  (`SceneComponent.K2_SetWorldRotation` _widgetdone (`KismetMathLibrary.MakeRotator` 0.0 0.0 (.yaw (`KismetMathLibrary.FindLookAtRotation` (`SceneComponent.K2_GetComponentLocation` _widgetdone) (`self.K2_GetActorLocation` (`GameplayStatics.GetPlayerCameraManager` 0))))) false false))

(fn `UserConstructionScript`
  (`TextRenderComponent.K2_SetText` (`self.LevelText`) (`KismetTextLibrary.Conv_IntToText` (`self.Level`))))